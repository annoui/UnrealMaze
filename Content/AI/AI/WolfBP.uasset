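; A wolf AI pawn that wanders randomly and hunts the first-person player when it sees them.
; While no enemy is seen, Tick waits a random delay and moves to a random reachable point nearby.
; PawnSensing triggers a chase, with a retriggerable delay clearing the sighting flag once the player is lost.
; Reaching the player shows the death widget and cursor, pauses the game and destroys the player.
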(event `self.ReceiveTick`
  (params (DeltaSeconds :type "Float (single-precision)"))
  ;[1 1 1] AI Random movement
  (if (not (`self.CanSeeEnemy?`))
    (`KismetSystemLibrary.Delay` (`KismetMathLibrary.RandomFloatInRange` 1.0 5.0))
    (set `self.IsMoving?` true)
    (`|AIMoveTo` self (`NavigationSystemV1.K2_GetRandomReachablePointInRadius` (`self.K2_GetActorLocation`) 1500.0 null null) null
      (:`OnSuccess`
        _)
      (:`OnFail`
        _))
    (set `self.IsMoving?` false)))

(event `self.PawnSensing.OnSeePawn`
  (params (Pawn :type "Pawn Object Reference"))
  (bind _asfirst_person_character (cast `/Game/FirstPersonBP/Blueprints/FirstPersonCharacter` Pawn))
  (`|ExecutionSequence`
    (:`then_0`
      (set `self.CanSeeEnemy?` true)
      (`|AIMoveTo` self (0.0 0.0 0.0) _asfirst_person_character
        (:`OnSuccess`
          (bind _returnvalue (`|CreateWidget` "/Game/HUD/DeathWidgetHUD.DeathWidgetHUD_C"))
          (`UserWidget.AddToViewport` _returnvalue 0)
          (set `PlayerController.bShowMouseCursor` true (`GameplayStatics.GetPlayerController` 0))
          (`GameplayStatics.SetGamePaused` true)
          (`self.K2_DestroyActor` _asfirst_person_character))))
    (:`then_1`
      (`KismetSystemLibrary.RetriggerableDelay` 0.5)
      (set `self.CanSeeEnemy?` false))))

(fn `UserConstructionScript`)